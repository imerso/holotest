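; BP_Boxes is an actor that recycles a physics cube once it falls out of the play area.
; Each Tick, a cube below a height threshold moves to a random position overhead, and its linear and angular velocities are zeroed so it drops afresh.
; A random rotation is computed during the reset but only written to a temporary quaternion, never applied to the cube.
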(event EventBeginPlay)

(event Collision|EventActorBeginOverlap
  (params (OtherActor :type Actor%20Object%20Reference)))

(event EventTick
  (params (DeltaSeconds :type Float%20%28single-precision%29))
  (bind _returnvalue (Math|Vector|MakeVector 0.0 0.0 0.0))
  (bind _returnvalue_2 (Math|Random|RandomFloat))
  (bind _returnvalue_3 (Math|Random|RandomFloat))
  (if (< (.Z (Math|Vector|BreakVector (Transformation|GetWorldLocation (Variables|Default|GetCube)))) -5e+01)
    (Transformation|SetWorldLocation (Variables|Default|GetCube) (Math|Vector|MakeVector (* (- _returnvalue_2 0.5) 6e+02) (* (- _returnvalue_3 0.5) 5e+02) (+ (* (Math|Random|RandomFloat) 5e+01) 4e+02)) false false)
    (Class|KismetMathLibrary|QuatSetfromEuler (Utilities|Struct|MakeQuat 0.0 0.0 0.0 1.0) (Math|Rotator|GetRotationXVector (Math|Rotator|MakeRotfromXY (Math|Conversions|ToVector(Float) _returnvalue_2) (Math|Conversions|ToVector(Float) _returnvalue_3))))
    (Class|PrimitiveComponent|SetAllPhysicsAngularVelocityinDegrees (Variables|Default|GetCube) _returnvalue false)
    (Physics|SetPhysicsLinearVelocity (Variables|Default|GetCube) _returnvalue false "None")))

(fn ConstructionScript)